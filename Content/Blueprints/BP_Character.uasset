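; Player character that moves along a single world axis, jumps, and flips gravity between down and up on left click.
; GravityChange toggles the movement component's gravity direction, while landing sets that direction to a zero vector.
; Death disables input, stops movement, fades the camera and uses a timer to respawn at NewCheckpoint with downward gravity.
; R restarts the level, and the start location is saved to SpawnPoint but not read here.
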(event `InputAxis|MoveRight`
  (params (AxisValue :type "Float (single-precision)"))
  ;[0.04502 0.04957 0.15 0.5] Movement and Jump
  (`self.AddMovementInput` (1.0 0.0 0.0) AxisValue))

(event `InputAction|Jump`
  (params (Key :type "Key Structure"))
  ;[0.04502 0.04957 0.15 0.5] Movement and Jump
  (:`Pressed`
    (`self.Jump`))
  (:`Released`
    (`self.StopJumping`)))

(event `self.ReceiveBeginPlay`
  (set `self.SpawnPoint` (`self.K2_GetActorLocation`)))

(event `Key|LeftMouseButton`
  (params (Key :type "Key Structure"))
  ;[0.15 0.1365 0.09076 0.5] Gravity Change
  (:`Pressed`
    (`self.Gravity Change`)))

(event `self.OnLanded`
  (params (Hit :type "HitResult Structure (by ref)"))
  ;[0.15 0.1365 0.09076 0.5] Gravity Change
  (`CharacterMovementComponent.SetGravityDirection` (`self.CharacterMovement`) (0.0 0.0 0.0)))

(event `Key|R`
  (params (Key :type "Key Structure"))
  ; Restart Level
  (:`Pressed`
    (`KismetSystemLibrary.ExecuteConsoleCommand` "Restartlevel" null)))

(event `/Game/Blueprints/I_Death.Death`
  ;[0.15 0.01391 0.01391 0.5] Player Death
  (`self.DisableInput` (`GameplayStatics.GetPlayerController` 0))
  (`MovementComponent.StopMovementImmediately` (`self.CharacterMovement`))
  (`PlayerCameraManager.StartCameraFade` :`self` (`GameplayStatics.GetPlayerCameraManager` 0) :`ToAlpha` 3.0 :`Duration` 3.2)
  (`KismetSystemLibrary.K2_SetTimerDelegate` (delegate `Respawn`) 2.9))

(event `Respawn`
  ;[0.15 0.01391 0.01391 0.5] Player Death
  (set `self.ToggleGravity` true)
  (`CharacterMovementComponent.SetGravityDirection` (`self.CharacterMovement`) (0.0 0.0 -1.0))
  (`self.K2_SetActorLocation` (`self.NewCheckpoint`))
  (`self.EnableInput` (`GameplayStatics.GetPlayerController` 0))
  (`self.K2_TeleportTo` (`self.NewCheckpoint`)))

(fn `Gravity Change`
  (if (`self.ToggleGravity`)
    (set `self.ToggleGravity` false)
    (`CharacterMovementComponent.SetGravityDirection` (`self.CharacterMovement`) (0.0 0.0 1.0))
    (else
      (set `self.ToggleGravity` true)
      (`CharacterMovementComponent.SetGravityDirection` (`self.CharacterMovement`) (0.0 0.0 -1.0)))))

(fn `UserConstructionScript`)